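; Global level builder that spawns a grid-based lawn of grass and fences from a gamestate and rebuilds it on Reset input.
; LoadState takes grid size from the original gamestate and copies it into a current gamestate.
; SetupLawn replaces grass actors and sets their levels, while SetupFences spawns fences from flattened edge arrays without removing old ones.
; BeginPlay is empty, and the initial setup chain is unwired.
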(event `self.ReceiveBeginPlay`)

(event `InputAction|Reset`
  (params (Key :type "Key Structure"))
  (:`Released`
    (`self.Reset`)))

(fn `LoadState`
  (params (GameState :type "/Game/GamestateBlueprint Object Reference"))
  (set `self.maxX` (`/Game/GamestateBlueprint.maxX` GameState))
  (set `self.maxY` (`/Game/GamestateBlueprint.maxY` GameState))
  (bind _output_get (set `self.OriginalGamestate` GameState))
  (if (not (`KismetSystemLibrary.IsValid` (`self.CurrentGamestate`)))
    (bind _returnvalue (`|SpawnActorFromClass` "/Game/GamestateBlueprint.GamestateBlueprint_C" (`KismetMathLibrary.MakeTransform` (0.0 0.0 0.0)) "Undefined" "OverrideRootScale" null null))
    (set `self.CurrentGamestate` _returnvalue))
  (`/Game/GamestateBlueprint.CopyState` (`self.CurrentGamestate`) _output_get))

(fn `Reset`
  (`self.LoadState` (`self.OriginalGamestate`))
  (`self.SetupLawn` (`self.maxX`) (`self.maxY`)))

(fn `SetupFences`
  (bind _originalgamestate (`self.OriginalGamestate`))
  (bind _maxy (`self.maxY`))
  (bind _maxy_2 (`self.maxY`))
  (bind _returnvalue (+ _maxy 1))
  (for (_array_element _array_index) (`/Game/GamestateBlueprint.VertFences` _originalgamestate)
    (if _array_element
      (`|SpawnActorFromClass` "/Game/FenceBlueprint.FenceBlueprint_C" (`KismetMathLibrary.MakeTransform` (`KismetMathLibrary.MakeVector` (* (- (`KismetMathLibrary.Conv_IntToDouble` (/ _array_index _returnvalue)) (* (- (`self.maxX`) 1) 0.5)) 110.0) (* (- (`KismetMathLibrary.Conv_IntToDouble` (mod _array_index _returnvalue)) (* _maxy 0.5)) 110.0) 100.0) (struct) (1.0 0.2 1.0)) "Undefined" "OverrideRootScale" null null)))
  (for (_array_element_2 _array_index_2) (`/Game/GamestateBlueprint.HorizFences` _originalgamestate)
    (if _array_element_2
      (`|SpawnActorFromClass` "/Game/FenceBlueprint.FenceBlueprint_C" (`KismetMathLibrary.MakeTransform` (`KismetMathLibrary.MakeVector` (* (- (`KismetMathLibrary.Conv_IntToDouble` (/ _array_index_2 _maxy_2)) (* (`self.maxX`) 0.5)) 110.0) (* (- (`KismetMathLibrary.Conv_IntToDouble` (mod _array_index_2 _maxy_2)) (* (- _maxy_2 1) 0.5)) 110.0) 100.0) (struct) (0.2 1.0 1.0)) "Undefined" "OverrideRootScale" null null))))

(fn `SetupLawn`
  (params (dimX :type Integer) (dimY :type Integer))
  (`self.SetupFences`)
  (for _array_element (`self.lawnArr`)
    (`self.K2_DestroyActor` _array_element))
  (bind (_current_point _total_points _0_1_phase _poly_center _x_row _y_row) (`/Engine/ArtTools/RenderToTexture/Macros/RenderToTextureMacros.2D Grid Execution Macro` 110.0 (0.0 0.0 0.0) dimX dimY)
    (:`Per Poly Execution`
      (bind _returnvalue (`|SpawnActorFromClass` "/Game/grass/GrassBlueprint.GrassBlueprint_C" (`KismetMathLibrary.Conv_VectorToTransform` _poly_center) "Undefined" "OverrideRootScale" null null))
      (bind _returnvalue_2 (+ _y_row (* _x_row dimY)))
      (`/Game/grass/GrassBlueprint.ChangeLevel` _returnvalue (`|GetArrayItem` (`/Game/GamestateBlueprint.GrassLevels` (`self.OriginalGamestate`)) _returnvalue_2))
      (`KismetArrayLibrary.Array_Set` (`self.lawnArr`) _returnvalue_2 _returnvalue true))))

(fn `UserConstructionScript`)